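; BP_AFLokimotive is the Blueprint for the Lokimotive vehicle, adding its horn.
; OnHonkBegin calls LokiHonk, which plays the Horn_AFLokimotive sound at the MMesh location with the driver as owning actor.
; The Possessed event is overridden with an empty body, and its parent call is left disconnected, so parent possession logic in that event does not run.
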(event EventBeginPlay
  (|CallParentFunction) ; This node is disabled and will not be called.\nDrag off pins to build functionality.
)

(event Collision|EventActorBeginOverlap
  (params (OtherActor :type Actor%20Object%20Reference))
  (|CallParentFunction OtherActor) ; This node is disabled and will not be called.\nDrag off pins to build functionality.
)

(event EventTick
  (params (DeltaSeconds :type Float%20%28single-precision%29))
  (|CallParentFunction DeltaSeconds) ; This node is disabled and will not be called.\nDrag off pins to build functionality.
)

(event EventPossessed
  (params (NewController :type Controller%20Object%20Reference))
  ;[1 1 1] yeetus
)

(event EventOnHonkBegin
  ;[1 1 1] yeetus
  (Vehicle|LokiHonk))

(fn ConstructionScript
  (|CallParentFunction))

(fn LokiHonk
  (Audio|PlaySoundatLocation "/AFChooPP/Vehicles/Loki/Horn_AFLokimotive.Horn_AFLokimotive" (Transformation|GetWorldLocation (Variables|Default|GetmMesh)) "0, 0, 0" 1.0 1.0 0.0 0 0 (Class|FGDriveablePawn|GetDriver))
  (return))